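; BP_XenomorphFollow is a xenomorph pawn that moves toward a set destination when its Jumpscare event is called.
; Jumpscare issues an AI MoveTo toward PointB and prints a debug message on success or failure.
; Disconnected nodes for playing the alien level sequence, playing a hatch seal sound and hiding a plane remain in the graph but never run.
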(event `self.Jumpscare`
  (`|ExecutionSequence`
    (:`then_1`
      (`|AIMoveTo` self (`self.PointB`) null
        (:`OnSuccess`
          (`KismetSystemLibrary.PrintString` "Hello"))
        (:`OnFail`
          (`KismetSystemLibrary.PrintString` "Can't Move"))))))

(fn `UserConstructionScript`)