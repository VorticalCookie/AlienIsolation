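; Hideable locker that the player interacts with, built on a parent hiding class, with a jumpscare for staying inside too long.
; Interact swings the door hinge open by timeline with a sound, then runs the parent interaction and starts a six-second timer.
; The HidingED dispatcher closes the door and re-enables interaction.
; If the player is still hiding when the timer fires, the door reopens and triggers the player's locker jumpscare.
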(event `self.ReceiveBeginPlay`
  (`parent.ReceiveBeginPlay`)
  (add `self.HidingED` (delegate `HidingED_Event`)))

(event `HidingED_Event`
  (`self.Close Door`))

(event `/Game/_Blueprints/BPI_Interaction.Interact`
  (if (`self.CanInteract`)
    (set `self.CanInteract` false)
    (bind (_direction _alpha) (`Timeline|OpenDoor` :!via `PlayFromStart`)
      (:`Update`
        (`|ExecutionSequence`
          (:`then_0`
            (`SceneComponent.K2_SetRelativeRotation` (`self.DoorHinge`) (`KismetMathLibrary.MakeRotator` 0.0 0.0 (`KismetMathLibrary.Lerp` 0.0 -100.0 _alpha)) false false))
          (:`then_1`
            (`/Engine/EditorBlueprintResources/StandardMacros.DoOnce` false :!label _label
              (:`Completed`
                (`GameplayStatics.PlaySoundAtLocation` "/Game/_VFX/Audio/Door/Locker_Close_HD.Locker_Close_HD" (0.0 0.0 0.0) (struct) 1.0 1.0 1.8 null null null null))))))
      (:`Finished`
        (`parent.Interact`)
        (`KismetSystemLibrary.K2_SetTimerDelegate` (delegate `CustomEvent`) 6.0)))))

(event `CustomEvent`
  (bind _playerref (`self.PlayerRef`))
  (if (`/Game/FirstPerson/Blueprints/BP_FirstPersonCharacter.IsHiding?` _playerref)
    (bind (_direction _alpha) (`Timeline|Timeline` :!via `PlayFromStart`)
      (:`Update`
        (`SceneComponent.K2_SetRelativeRotation` (`self.DoorHinge`) (`KismetMathLibrary.MakeRotator` 0.0 0.0 (`KismetMathLibrary.Lerp` 0.0 -100.0 _alpha)) false false)
        (`/Engine/EditorBlueprintResources/StandardMacros.DoOnce` false
          (:`Completed`
            (`GameplayStatics.PlaySoundAtLocation` "/Game/_VFX/Audio/Door/Locker_Close_HD.Locker_Close_HD" (0.0 0.0 0.0) (struct) 1.0 1.0 1.8 null null null null)
            (`KismetSystemLibrary.Delay` 0.6)
            (`/Game/FirstPerson/Blueprints/BP_FirstPersonCharacter.LockerJumpscare` _playerref)))))))

(event `Close Door`
  (bind (_direction _alpha) (`Timeline|ClosedLockerDoor` :!via `PlayFromStart`)
    (:`Update`
      (`SceneComponent.K2_SetRelativeRotation` (`self.DoorHinge`) (`KismetMathLibrary.MakeRotator` 0.0 0.0 (`KismetMathLibrary.Lerp` -100.0 0.0 _alpha)) false false))
    (:`Finished`
      (set `self.CanInteract` true)
      (goto _label :!via `Reset`))))

(fn `UserConstructionScript`
  (`parent.UserConstructionScript`))