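; Xenomorph actor that performs a one-time jumpscare run when its Jumpscare event is called.
; It moves to PointB via AIMoveTo while a footsteps sound, spawned at its starting location, plays.
; On arrival it stops the footsteps, plays a spatialized hatch-seal sound and hides its Plane; a failed move only prints a debug message.
; An AlienSequence level sequence playback is present but unconnected.
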(event `/Game/_Blueprints/BPI_Jumpscare.Jumpscare`
  (`/Engine/EditorBlueprintResources/StandardMacros.DoOnce` false
    (:`Completed`
      (`|AIMoveTo` self (`self.PointB`) null
        (:`then`
          (bind _returnvalue (`GameplayStatics.SpawnSoundAtLocation` "/Game/_VFX/Audio/Alien_Footsteps_Metal_V3_2_08_-_MattFiler_-_SoundLoadMate_com.Alien_Footsteps_Metal_V3_2_08_-_MattFiler_-_SoundLoadMate_com" (`self.K2_GetActorLocation` self) (struct) 0.4 1.0 0.0 "/Game/_VFX/SoundAttenuationSpatial.SoundAttenuationSpatial" null))
          (set `self.FootSteps` _returnvalue))
        (:`OnSuccess`
          (`AudioComponent.Stop` (`self.FootSteps`))
          (`GameplayStatics.PlaySoundAtLocation` "/Game/_VFX/Audio/hatch-seal-104129.hatch-seal-104129" (`self.K2_GetActorLocation` self) (struct) 1.0 1.0 3.0 "/Game/_VFX/SoundAttenuationSpatial.SoundAttenuationSpatial" null null null)
          (`SceneComponent.SetVisibility` (`self.Plane`) false false))
        (:`OnFail`
          (`KismetSystemLibrary.PrintString` "Can't Move"))))))

(fn `UserConstructionScript`)